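; Game state for the Macbeth game that switches music and player movement mode as the player enters the bar, basement, witch, parkour and arcade areas.
; On BeginPlay it resets progress flags, caches the Macbeth character and binds a handler to each area event.
; Handlers fade out current music and start the area's track.
; Bar and witch set a slow walk with narrower FOV; parkour and arcade set a faster run with wider FOV.
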(event `EnterBar_Event`
  (bind _ost (`self.OST`))
  (bind _idleost (`self.idleOST`))
  (`|ExecutionSequence`
    (:`then_0`
      (`/Engine/EditorBlueprintResources/StandardMacros.IsValid` _idleost :!label _label
        (:`Is Valid`
          (`AudioComponent.FadeOut` _idleost 0.5 0.0 "Linear"))
        (:`Is Not Valid`
          _))
      (`/Engine/EditorBlueprintResources/StandardMacros.IsValid` _ost
        (:`Is Valid`
          (`AudioComponent.FadeOut` _ost 0.5 0.0 "Linear"))))
    (:`then_1`
      (bind _returnvalue (`GameplayStatics.SpawnSound2D` "/Game/Macbeth/idle.idle" 0.02 1.0 0.0 null))
      (set `self.idleOST` _returnvalue))
    (:`then_2`
      (set `self.speedScale` 0.15 :!label _label_2)
      (`CameraComponent.SetFieldOfView` (`/Game/Macbeth/sprite/char/bigmac/Macbeth_Char.SideViewCameraComponent` (`self.macbeth`)) 90.0)
      (set `self.isRun` false))))

(event `EnterBasement_Event`
  (`|ExecutionSequence`
    (:`then_0`
      (goto _label))
    (:`then_1`
      (goto _label))
    (:`then_2`
      (bind _returnvalue (`GameplayStatics.SpawnSound2D` "/Game/Macbeth/bassment.bassment" 0.1 1.0 0.0 null :!label _label_3))
      (set `self.OST` _returnvalue))))

(event `self.ReceiveBeginPlay`
  (set `self.talkedToFrog` false)
  (set `self.talkedToVVitch` false)
  (set `self.inRangeForAnim` false)
  (set `self.isRun` false)
  (set `self.speedScale` 0.15)
  (bind _asmacbeth_char (cast `/Game/Macbeth/sprite/char/bigmac/Macbeth_Char` (`GameplayStatics.GetPlayerCharacter` 0)))
  (set `self.macbeth` _asmacbeth_char)
  (`|ExecutionSequence`
    (:`then_0`
      (add `self.EnterBar` (delegate `EnterBar_Event`)))
    (:`then_1`
      (add `self.EnterBasement` (delegate `EnterBasement_Event`)))
    (:`then_2`
      (add `self.EnterVVitch` (delegate `EnterVVitch_Event`)))
    (:`then_3`
      (add `self.EnterParkour` (delegate `EnterParkour_Event`)))
    (:`then_4`
      (add `self.EnterArcade` (delegate `EnterArcade_Event`)))))

(event `EnterVVitch_Event`
  (`|ExecutionSequence`
    (:`then_0`
      (goto _label))
    (:`then_1`
      (goto _label_2))
    (:`then_2`
      (goto _label_3))))

(event `EnterArcade_Event`
  (`|ExecutionSequence`
    (:`then_0`
      (goto _label))
    (:`then_1`
      (set `self.speedScale` 0.7 :!label _label_4)
      (`CameraComponent.SetFieldOfView` (`/Game/Macbeth/sprite/char/bigmac/Macbeth_Char.SideViewCameraComponent` (`self.macbeth`)) 130.0)
      (set `self.isRun` true))
    (:`then_2`
      (bind _returnvalue (`GameplayStatics.SpawnSound2D` "/Game/Macbeth/COH_-_A.COH_-_A" 0.06 1.0 0.0 null))
      (set `self.OST` _returnvalue))))

(event `EnterParkour_Event`
  (`|ExecutionSequence`
    (:`then_0`
      (goto _label))
    (:`then_1`
      (goto _label_4))
    (:`then_2`
      (bind _returnvalue (`GameplayStatics.SpawnSound2D` "/Game/Macbeth/podval_parkur.podval_parkur" 0.02 1.0 0.0 null))
      (set `self.OST` _returnvalue))))

(fn `UserConstructionScript`)